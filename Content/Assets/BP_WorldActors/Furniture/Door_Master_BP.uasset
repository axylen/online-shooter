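; Master Blueprint for a physics door with configurable door and doorjamb meshes, pushed by point damage.
; Construction sets both meshes, then CanBeOpen drives the door's physics simulation and the actor's replication.
; Point damage on a simulating component of an openable door triggers a server-to-multicast rotation sync, then a multicast impulse along the hit direction.
; The impulse scales with damage up to a cap and is applied as a velocity change, ignoring mass.
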(event `MC_ApplyImpulse`
  (params (Target :type "PrimitiveComponent Object Reference") (Impulse :type "Vector Structure"))
  (`PrimitiveComponent.AddImpulse` Target Impulse "None" true))

(event `MC_FixRotation`
  (params (NewRotation :type "Rotator Structure"))
  (`SceneComponent.K2_SetWorldRotation` (`self.Door`) NewRotation false false))

(event `Server_FixRotation`
  (`self.MC_FixRotation` (`SceneComponent.K2_GetComponentRotation` (`self.Door`))))

(event `self.ReceivePointDamage`
  (params (Damage :type "Float (single-precision)") (DamageType :type "DamageType Object Reference") (HitLocation :type "Vector Structure") (HitNormal :type "Vector Structure") (HitComponent :type "PrimitiveComponent Object Reference") (BoneName :type Name) (ShotFromDirection :type "Vector Structure") (InstigatedBy :type "Controller Object Reference") (DamageCauser :type "Actor Object Reference") (HitInfo :type "HitResult Structure (by ref)"))
  (bind (_start _end) (`/Game/Blueprints/BP/Library/BP_Funtion_Library.GetHitStartAndEnd` HitInfo))
  (`/Game/Blueprints/BP/Library/Object_Macro_Library.SimulatingPhysics` HitComponent
    (:`true`
      (if (`self.CanBeOpen`)
        (`self.Server_FixRotation`)
        (`self.MC_ApplyImpulse` HitComponent (* (`KismetMathLibrary.GetDirectionUnitVector` _start _end) (`KismetMathLibrary.FClamp` (* Damage 50.0) 0.0 1000.0)))))))

(fn `SetupCanBeOpen`
  (`PrimitiveComponent.SetSimulatePhysics` (`self.Door`) (`self.CanBeOpen`))
  (`self.SetReplicates` self (`self.CanBeOpen`)))

(fn `UserConstructionScript`
  (`parent.UserConstructionScript`)
  (`StaticMeshComponent.SetStaticMesh` (`self.Door`) (`self.DoorMesh`))
  (`StaticMeshComponent.SetStaticMesh` (`self.Doorjamb`) (`self.DoorjambMesh`))
  (`self.SetupCanBeOpen`))