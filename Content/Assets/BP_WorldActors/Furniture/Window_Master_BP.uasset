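; Master window Blueprint with an optional frame mesh and glass that is either breakable or static.
; The construction script adds a static glass mesh or, for breakable unbroken windows, a destructible component with a random mesh, re-rolled on BeginPlay.
; Point damage on that component triggers MC_Damage, applying fixed damage along the hit trace, playing a shatter sound and destroying the Box component.
; IsBroken then marks the window broken, which setup respects.
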(event `self.ReceiveBeginPlay`
  (`self.SetupDestrMesh`))

(event `self.ReceivePointDamage`
  (params (Damage :type "Float (single-precision)") (DamageType :type "DamageType Object Reference") (HitLocation :type "Vector Structure") (HitNormal :type "Vector Structure") (HitComponent :type "PrimitiveComponent Object Reference") (BoneName :type Name) (ShotFromDirection :type "Vector Structure") (InstigatedBy :type "Controller Object Reference") (DamageCauser :type "Actor Object Reference") (HitInfo :type "HitResult Structure (by ref)"))
  (bind (_start _end) (`/Game/Blueprints/BP/Library/BP_Funtion_Library.GetHitStartAndEnd` HitInfo))
  (if (== HitComponent (`self.Destr_mesh`))
    (`self.MC_Damage` 75.0 HitLocation (`KismetMathLibrary.GetDirectionUnitVector` _start _end))
    (set `self.IsBroken` true)))

(event `MC_Damage`
  (params (DamageAmount :type "Float (double-precision)") (HitLocation :type "Vector Structure (by ref)") (ImpulseDir :type "Vector Structure (by ref)"))
  (`DestructibleComponent.ApplyDamage` (`self.Destr_mesh`) DamageAmount HitLocation ImpulseDir 1.0)
  (`GameplayStatics.PlaySoundAtLocation` "/Game/Sounds/Shoted/Glass/glass_broken_Cue.glass_broken_Cue" HitLocation)
  (bind _box (`self.Box`)
    (:`then`
      (`ActorComponent.K2_DestroyComponent` _box))
    (:`else`)))

(fn `GetRandomDestrMesh`
  (returns (Item :type "DestructibleMesh Object Reference"))
  (return (`/Game/Blueprints/BP/Library/Object_Macro_Library.GetRandomItemOfArray` (`self.DestrMeshes`))))

(fn `SetupDestrMesh`
  (locals (_InnerMat :type "MaterialInstance Object Reference" :default "MaterialInstanceConstant'/Game/Materials/Materials/Materials/Glass/MAT_Glass_2.MAT_Glass_2'"))
  (bind _destr_mesh (`self.Destr_mesh`))
  (if (`self.IsBroken`)
    (bind _box (`self.Box`)
      (:`then`
        (`ActorComponent.K2_DestroyComponent` _box))
      (:`else`))
    (else
      (`/Engine/EditorBlueprintResources/StandardMacros.IsValid` (`self.Destr_mesh`)
        (:`Is Valid`
          (`DestructibleComponent.SetDestructibleMesh` _destr_mesh (`self.GetRandomDestrMesh`))
          (`PrimitiveComponent.SetMaterial` _destr_mesh 0 (`self.GlassMat`))
          (`PrimitiveComponent.SetMaterial` _destr_mesh 1 (`local._InnerMat`)))))))

(fn `UserConstructionScript`
  (bind _frame (`self.Frame`))
  (`parent.UserConstructionScript`)
  (`|ExecutionSequence`
    (:`then_0`
      (bind _framemesh (`self.FrameMesh`)
        (:`then`
          (`StaticMeshComponent.SetStaticMesh` _frame _framemesh)
          (`SceneComponent.SetVisibility` _frame true false))
        (:`else`
          (`SceneComponent.SetVisibility` _frame false false))))
    (:`then_1`
      (if (`self.CanBreak`)
        (if (`self.IsBroken`)
          (bind _box (`self.Box`)
            (:`then`
              (`ActorComponent.K2_DestroyComponent` _box))
            (:`else`))
          (else
            (bind _returnvalue (`AddComponent|NODE_AddDestructibleComponent-2`))
            (set `self.Destr_mesh` _returnvalue)
            (`self.SetupDestrMesh`)))
        (else
          (bind _returnvalue_2 (`AddComponent|NODE_AddStaticMeshComponent-2`))
          (`StaticMeshComponent.SetStaticMesh` _returnvalue_2 "/Game/Assets/3DModels/Furniture/Windows/Glass.Glass")
          (`PrimitiveComponent.SetMaterial` _returnvalue_2 0 (`self.GlassMat`)))))))