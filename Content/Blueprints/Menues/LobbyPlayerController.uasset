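; Player controller for the multiplayer lobby that connects each player's menu to LobbyGamemode for chat, player list and map voting.
; Initial setup loads or creates saved player settings with a default loadout, opens the UI-only lobby widget, and has the authority generate the map list.
; Server events forward messages and votes to the game mode, while other events push updates into the widget.
; On EndPlay, remote instances destroy the session, then call the vote event with -1.
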(event `Server_SendMessage`
  (params (Msg :type Text))
  ;[1 1 1] Chat
  (bind _aslobby_gamemode (cast `/Game/Blueprints/Menues/LobbyGamemode` (`GameplayStatics.GetGameMode`)))
  (`/Game/Blueprints/Menues/LobbyGamemode.Server_Upd_Chat` _aslobby_gamemode Msg))

(event `InitialSetup`
  (`WidgetLayoutLibrary.RemoveAllWidgets`)
  (`self.Init`)
  (`/Engine/EditorBlueprintResources/ActorMacros.Switch Has Authority`
    (:`Authority`
      (bind _aslobby_gamemode (cast `/Game/Blueprints/Menues/LobbyGamemode` (`GameplayStatics.GetGameMode`)))
      (`/Game/Blueprints/Menues/LobbyGamemode.GenerateMapList` _aslobby_gamemode))))

(event `self.ReceiveEndPlay`
  (params (EndPlayReason :type "EEndPlayReason Enum" :default "Destroyed"))
  (`/Engine/EditorBlueprintResources/ActorMacros.Switch Has Authority`
    (:`Remote`
      (`DestroySessionCallbackProxy.DestroySession` self
        (:`then`
          (`self.Server_OnMapVote` -1))))))

(event `GetMessage`
  (params (Msg :type Text))
  ;[1 1 1] Chat
  (`/Game/UMG/Widgets/Chat.AddMessage` (`/Game/UMG/Menu/LobbyMenu.Chat` (`self.LobbyWB`)) Msg))

(event `OnGameStart`
  (params (MapID :type Integer) (Gamemode :type "/Game/Blueprints/BP/ENUMS/E_Gamemods Enum"))
  (`/Game/Blueprints/BP/Library/BP_Funtion_Library.ShowLoadingScreen` self))

(event `UpdateLobbySettings`
  (params (Map :type "Array of /Game/Maps/SelectedMap_Struct Structure"))
  (bind _lobbywb (`self.LobbyWB`))
  ;[1 1 1] Обновление настроек игры
  (`/Engine/EditorBlueprintResources/StandardMacros.IsValid` _lobbywb
    (:`Is Valid`
      (set `/Game/UMG/Menu/LobbyMenu.Maps` Map _lobbywb)
      (`/Game/UMG/Menu/LobbyMenu.Local_CreateMapList` _lobbywb)
      (set `self.VotedMap` -1))))

(event `Server_OnMapVote`
  (params (Map :type Integer))
  (`/Game/Blueprints/Menues/LobbyGamemode.NewMapVote` (cast `/Game/Blueprints/Menues/LobbyGamemode` (`GameplayStatics.GetGameMode`) :!pure true) (`self.VotedMap`) Map)
  (set `self.VotedMap` Map))

(event `AddPlayerInfo`
  (params (Names :type "Array of String"))
  (bind _lobbywb (`self.LobbyWB`))
  ;[1 1 1] Создаёт список игроков
  (`/Engine/EditorBlueprintResources/StandardMacros.IsValid` _lobbywb
    (:`Is Valid`
      (`/Game/UMG/Menu/LobbyMenu.CreatePlayerList` _lobbywb Names))))

(event `UpdateMapVoting`
  (params (Votes :type "Array of Integer (by ref)"))
  (`/Game/UMG/Menu/LobbyMenu.UpdateMapVotes` (`self.LobbyWB`) Votes))

(fn `GetPlayerSettings`
  (params (SlotName :type String :default "PlayerSettings"))
  (returns (GameSave :type "/Game/Blueprints/Settings/PlayerGameSave Object Reference"))
  (locals (_SlotName :type String) (_GameSave :type "/Game/Blueprints/Settings/PlayerGameSave Object Reference"))
  (bind _output_get (set `local._SlotName` SlotName))
  (bind _returnvalue (`GameplayStatics.DoesSaveGameExist` _output_get)) ; Существует ли сохранение с текущим именем
  (if _returnvalue
    (bind _returnvalue_2 (`GameplayStatics.LoadGameFromSlot` (`local._SlotName`))) ; Загружает сохранение
    (set `local._GameSave` (cast `/Game/Blueprints/Settings/PlayerGameSave` _returnvalue_2 :!pure true))
    (else
      (bind _returnvalue_3 (`GameplayStatics.CreateSaveGameObject` "/Game/Blueprints/Settings/PlayerGameSave.PlayerGameSave_C")) ; Создаёт файл сохранения
      (set `local._GameSave` (cast `/Game/Blueprints/Settings/PlayerGameSave` _returnvalue_3 :!pure true))
      (set `/Game/Blueprints/Settings/PlayerGameSave.Settings` (make `/Game/Blueprints/Settings/PlayerSettings` "/Game/Items/Weapon/Primary/AKM/AKM_BP.AKM_BP_C" "/Game/Items/Weapon/Secondary/M9/M9_BP.M9_BP_C" "/Game/Items/Clotch/Hats/Hair_1/Hat_Hair.Hat_Hair_C" "/Game/Items/Clotch/Glasses/Glasses_Master_BP.Glasses_Master_BP_C" "/Game/Items/Clotch/Tops/ACU_Rolled_Up/Top_ACU_Rolled_Up.Top_ACU_Rolled_Up_C" "/Game/Items/Clotch/Gloves/Gloves_Master_BP.Gloves_Master_BP_C" "/Game/Items/Clotch/Pants/TacticalResponse/Pants_TacticalResponse.Pants_TacticalResponse_C" "/Game/Items/Clotch/Shoes/Canvas/Shoes_Canvas.Shoes_Canvas_C") (`local._GameSave`))
      (`/Game/Blueprints/BP/Library/Object_Macro_Library.SavePlayerSettings` (`local._GameSave`) (`local._SlotName`))))
  (return (`local._GameSave`)))

(fn `Init`
  (bind _asshooter_gameinstance (cast `/Game/Blueprints/ShooterGameinstance` (`GameplayStatics.GetGameInstance`))
    (:`then`
      _)
    (:`CastFailed`
      _))
  (set `self.GameInstanceRef` _asshooter_gameinstance) ; Ссылка на GameInstance
  (set `self.PlayerSettings` (`self.GetPlayerSettings` "PlayerSettings"))
  (`self.SetupLobbyMenu`) ; Создание меню
)

(fn `SetupLobbyMenu`
  (`/Engine/EditorBlueprintResources/StandardMacros.IsValid` (`self.LobbyWB`)
    (:`Is Valid`
      _)
    (:`Is Not Valid`
      (bind _returnvalue (`|CreateWidget` "/Game/UMG/Menu/LobbyMenu.LobbyMenu_C" self))
      (bind _output_get (set `self.LobbyWB` _returnvalue))))
  (`UserWidget.AddToViewport` _output_get 0)
  (set `self.bShowMouseCursor` true)
  (`WidgetBlueprintLibrary.SetInputMode_UIOnlyEx` self (`self.LobbyWB`)))

(fn `UserConstructionScript`)