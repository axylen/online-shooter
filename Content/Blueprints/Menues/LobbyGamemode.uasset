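; Multiplayer lobby game mode that manages connected players, chat and map voting before a match.
; Joins, controller swaps and logouts update the controller list; the server pushes names, settings, vote counts and chat to every LobbyPlayerController.
; It builds a random list of map and gamemode pairs and tallies changeable votes.
; At start it picks randomly among top-voted entries, stores the gamemode in ShooterGameinstance, notifies players and server-travels to the map.
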(event `Server_Upd_Chat`
  (params (Msg :type Text))
  (for _array_element (`self.AllPlayerControllers`)
    (`/Game/Blueprints/Menues/LobbyPlayerController.GetMessage` _array_element Msg)))

(event `self.K2_OnSwapPlayerControllers`
  (params (OldPC :type "PlayerController Object Reference") (NewPC :type "PlayerController Object Reference"))
  (`self.PlayerConnected` NewPC))

(event `Start`
  (params (MapName :type String))
  (`KismetSystemLibrary.ExecuteConsoleCommand` (`KismetStringLibrary.Concat_StrStr` "servertravel /Game/Maps/InGame/" MapName) (`GameplayStatics.GetPlayerController` 0)))

(event `self.K2_PostLogin`
  (params (NewPlayer :type "PlayerController Object Reference"))
  (`/Engine/EditorBlueprintResources/ActorMacros.Switch Has Authority` ; Выполняется на сервере
    (:`Authority`
      (`self.PlayerConnected` NewPlayer))))

(event `UpdatePlayerList`
  ;[1 1 1] Обновляет список имён игроков
  (`KismetArrayLibrary.Array_Clear` (`self.AllPlayerNames`))
  (for _array_element (`self.AllPlayerControllers`)
    (`KismetArrayLibrary.Array_Add` (`self.AllPlayerNames`) (`PlayerState.PlayerName` (`Controller.PlayerState` _array_element))))
  (for _array_element_2 (`self.AllPlayerControllers`)
    (`/Game/Blueprints/Menues/LobbyPlayerController.AddPlayerInfo` _array_element_2 (`self.AllPlayerNames`))))

(event `self.K2_OnLogout`
  (params (ExitingController :type "Controller Object Reference"))
  ;[1 1 1] Обновляет список игроков при выходе игрока
  (bind _aslobby_player_controller (cast `/Game/Blueprints/Menues/LobbyPlayerController` ExitingController))
  (`KismetArrayLibrary.Array_RemoveItem` (`self.AllPlayerControllers`) _aslobby_player_controller)
  (`self.UpdatePlayerList`)
  (`/Game/Blueprints/Menues/LobbyPlayerController.Server_OnMapVote` _aslobby_player_controller -1))

(event `Update_MapVoteCount`
  (for _array_element (`self.AllPlayerControllers`)
    (`/Game/Blueprints/Menues/LobbyPlayerController.UpdateMapVoting` _array_element (`self.Votes`))))

(fn `GenerateMapList`
  (locals (_MapCount :type Integer :default 2) (_MapList :type "Array of /Game/Maps/Map_Struct Structure") (_Map :type "/Game/Maps/Map_Struct Structure") (GameinstanceRef :type "/Game/Blueprints/ShooterGameinstance Object Reference"))
  (bind _asshooter_gameinstance (cast `/Game/Blueprints/ShooterGameinstance` (`GameplayStatics.GetGameInstance`)))
  (set `local.GameinstanceRef` _asshooter_gameinstance)
  (set `local._MapList` (`/Game/Blueprints/ShooterGameinstance.MapList` _asshooter_gameinstance))
  (`KismetArrayLibrary.Array_Clear` (`self.MapList`))
  (for _ (range 1 (+ (`local._MapCount`) 1))
    (set `local._Map` (`KismetArrayLibrary.Array_Get` (`local._MapList`) (`KismetMathLibrary.RandomIntegerInRange` 0 (`KismetArrayLibrary.Array_LastIndex` (`local._MapList`))))) ; Случайная карта
    (`KismetArrayLibrary.Array_Add` (`self.MapList`) (make `/Game/Maps/SelectedMap_Struct` (`KismetArrayLibrary.Array_Find` (`/Game/Blueprints/ShooterGameinstance.MapList` (`local.GameinstanceRef`)) (`local._Map`)) (select `int` (`KismetMathLibrary.RandomIntegerInRange` 0 1) :`0` "NewEnumerator1" :`1` "NewEnumerator0" :!type "/Game/Blueprints/BP/ENUMS/E_Gamemods Enum"))) ; Добавляет текущую карту с режимом игры к списку
    (`KismetArrayLibrary.Array_RemoveItem` (`local._MapList`) (`local._Map`)) ; Удаляет выбранную карту из списка
  )
  (`self.UpdateGameSettings`) ; Обновляет список карт в голосовании
)

(fn `GetGameinst`
  (returns (`Shooter Gameinstance` :type "/Game/Blueprints/ShooterGameinstance Object Reference"))
  (bind _asshooter_gameinstance (cast `/Game/Blueprints/ShooterGameinstance` (`GameplayStatics.GetGameInstance`)))
  (return _asshooter_gameinstance))

(fn `NewMapVote`
  (params (Old :type Integer) (New :type Integer))
  (locals (_New :type Integer) (_Old :type Integer :default -1))
  (set `local._Old` Old)
  (set `local._New` New)
  (if (>= (`local._Old`) 0)
    (`/Game/Blueprints/BP/Library/Object_Macro_Library.ChangeArrElem` (`self.Votes`) (`local._Old`) -1 true) ; Убирает предыдущий голос
    (`/Game/Blueprints/BP/Library/Object_Macro_Library.ChangeArrElem` (`self.Votes`) (`local._New`) 1 true :!label _label) ; Добавляет голос
    (elif (>= (`local._New`) 0)
      (goto _label)
      (else
        (`/Game/Blueprints/BP/Library/Object_Macro_Library.ChangeArrElem` (`self.Votes`) (`local._Old`) -1 true) ; Убирает предыдущий голос
      )))
  (`self.Update_MapVoteCount`) ; Обновляет кол-во голосов
)

(fn `PlayerConnected`
  (params (Player :type "PlayerController Object Reference"))
  (bind _aslobby_player_controller (cast `/Game/Blueprints/Menues/LobbyPlayerController` Player)
    (:`then`
      (`KismetArrayLibrary.Array_AddUnique` (`self.AllPlayerControllers`) _aslobby_player_controller)
      (`/Game/Blueprints/Menues/LobbyPlayerController.InitialSetup` _aslobby_player_controller) ; Первоначальная настройка
      (`/Game/Blueprints/Menues/LobbyPlayerController.UpdateLobbySettings` _aslobby_player_controller (`self.MapList`)) ; Устанавливат информацию об игре
      (`self.UpdatePlayerList`) ; Обновляет список игроков
      (`/Game/Blueprints/Menues/LobbyPlayerController.UpdateMapVoting` _aslobby_player_controller (`self.Votes`)))
    (:`CastFailed`
      (`KismetSystemLibrary.PrintString` "cast failed. Controller" true true (struct :`G` 0.66 :`B` 1.0 :`A` 1.0) 20.0))))

(fn `SelectMapOnStartGame`
  (returns (Map :type "/Game/Maps/Map_Struct Structure") (Gamemode :type "/Game/Blueprints/BP/ENUMS/E_Gamemods Enum") (ID :type Integer))
  (locals (_MaxList :type "Array of Integer") (_MaxV :type Integer))
  (bind _item (`/Game/Blueprints/BP/Library/Object_Macro_Library.GetRandomItemOfArray` (`local._MaxList`)))
  (bind (_item_mapid _item_gamemode) (break `/Game/Maps/SelectedMap_Struct` (`KismetArrayLibrary.Array_Get` (`self.MapList`) _item)))
  (set `local._MaxList` (`.Index` (`/Game/Blueprints/BP/Library/Get_Library.GetMaxIntOfArray` (`self.Votes`))))
  (return (`/Game/Blueprints/BP/Library/BP_Funtion_Library.GetMapByID` _item_mapid) _item_gamemode _item))

(fn `StartTheGame`
  (locals (_Gamemode :type "/Game/Blueprints/BP/ENUMS/E_Gamemods Enum" :default "NewEnumerator1") (_MapID :type Integer :default 0))
  (bind (_map _gamemode _id) (`self.SelectMapOnStartGame`))
  (set `local._Gamemode` _gamemode)
  (set `local._MapID` _id)
  (set `/Game/Blueprints/ShooterGameinstance.Gamemode` (`local._Gamemode`) (`self.GetGameinst`))
  (for _array_element (`self.AllPlayerControllers`)
    (`/Game/Blueprints/Menues/LobbyPlayerController.OnGameStart` _array_element (`local._MapID`) (`local._Gamemode`)))
  (`KismetSystemLibrary.ExecuteConsoleCommand` (`KismetStringLibrary.Concat_StrStr` "servertravel /Game/Maps/InGame/" (`.MapName_6_3883F4004B55E9B3FB73BD8F865E1B8C` (break `/Game/Maps/Map_Struct` _map))) (`GameplayStatics.GetPlayerController` 0)))

(fn `UpdateGameSettings`
  (`KismetArrayLibrary.Array_Clear` (`self.Votes`))
  (for _array_element (`self.AllPlayerControllers`)
    (`/Game/Blueprints/Menues/LobbyPlayerController.UpdateLobbySettings` _array_element (`self.MapList`))))

(fn `UserConstructionScript`)