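; Player controller for the multiplayer shooter, managing spawning, match UI, saved settings and camera effects.
; Server events spawn and possess either a spawn camera or a ShooterCharacter built from PlayerSettings, using randomly picked placed spawn actors.
; It shows respawn, scoreboard and aftermath widgets, disabling input at match end.
; Construction loads sensitivity and mouse inversion from a save slot, creating a default loadout if absent; camera helpers handle fades and interpolated FOV.
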(event `OWN_UpdScore`
  (bind _scorewb (`self.ScoreWB`))
  (`KismetSystemLibrary.Delay` 0.45)
  (`/Engine/EditorBlueprintResources/StandardMacros.IsValid` _scorewb
    (:`Is Valid`
      (if (`Widget.IsVisible` _scorewb)
        (`/Game/UMG/Widgets/Scores_UMG.UpdateScore` (`/Game/UMG/InGameInterface/ScoreBoard.Scores` _scorewb))))))

(event `FadeCam`
  (params (FromAlpha :type "Float (double-precision)" :default 1.0) (ToAlpha :type "Float (double-precision)" :default 0.0) (Duration :type "Float (double-precision)" :default 0.25))
  (if (`self.IsLocalController`)
    (`PlayerCameraManager.StartCameraFade` :`self` (`GameplayStatics.GetPlayerCameraManager` 0) :`FromAlpha` FromAlpha :`ToAlpha` ToAlpha :`Duration` Duration :`bShouldFadeAudio` true :`bHoldWhenFinished` true)))

(event `OWN_OnMatchEnded`
  (params (WinnerText :type Text))
  (bind _returnvalue (`self.K2_GetPawn` self))
  (`self.ShowAftermathUMG` WinnerText)
  (`self.DisableInput` _returnvalue self)
  (`self.DisableInput` self self)
  (bind _asshooter_character (cast `/Game/Character/ShooterCharacter` _returnvalue))
  (`/Game/Character/ShooterCharacter.Server_WantToShoot` _asshooter_character false))

(event `InitialSetup`
  (set `self.bShowMouseCursor` true)
  (`KismetSystemLibrary.Delay` 0.2)
  (`self.Server_SpawnCamera`)
  (`WidgetLayoutLibrary.RemoveAllWidgets`)
  (if (not (`self.IsMathEnded`))
    (`self.ShowRespawnMenu`)))

(event `Server_SetPlayerSettings`
  (params (PlayerSettings :type "/Game/Blueprints/Settings/PlayerSettings Structure"))
  (set `self.PlayerSettings` PlayerSettings))

(event `InputAction|ShowScore`
  (params (Key :type "Key Structure" :default "AnyKey"))
  (:`Pressed`
    (`self.CreateScoreList`))
  (:`Released`
    (`/Engine/EditorBlueprintResources/StandardMacros.IsValid` (`self.ScoreWB`)
      (:`Is Valid`
        (`Widget.RemoveFromParent` (`self.ScoreWB`))))))

(event `Server_SpawnPlayer`
  ;[1 1 1] Спавн
  (bind _outactors (`GameplayStatics.GetAllActorsOfClass` "/Game/MapComponents/Spawn/PlayerSpawnPos.PlayerSpawnPos_C"))
  (bind (_returnvalue_location _returnvalue_rotation) (`KismetMathLibrary.BreakTransform` (`self.GetTransform` (`KismetArrayLibrary.Array_Get` _outactors (`KismetMathLibrary.RandomIntegerInRange` 0 (`KismetArrayLibrary.Array_LastIndex` _outactors))))))
  (bind _returnvalue (`|SpawnActorFromClass` "/Game/Character/ShooterCharacter.ShooterCharacter_C" (`KismetMathLibrary.MakeTransform` _returnvalue_location _returnvalue_rotation (1.0 1.0 1.0)) "Undefined" "OverrideRootScale" null (`self.PlayerSettings`)))
  (`/Engine/EditorBlueprintResources/StandardMacros.IsValid` _returnvalue
    (:`Is Valid`
      (`CameraComponent.SetFieldOfView` (`/Game/Character/ThirdPersonCharacterAnim.Camera` _returnvalue) (`self.CameraFOV`))
      (`self.Possess` _returnvalue))))

(event `Server_SpawnCamera`
  ;[1 1 1] Спавн
  (bind _outactors (`GameplayStatics.GetAllActorsOfClass` "/Game/MapComponents/Spawn/SpawnCameraPos.SpawnCameraPos_C"))
  (bind (_returnvalue_location _returnvalue_rotation) (`KismetMathLibrary.BreakTransform` (`self.GetTransform` (`KismetArrayLibrary.Array_Get` _outactors (`KismetMathLibrary.RandomIntegerInRange` 0 (`KismetArrayLibrary.Array_LastIndex` _outactors))))))
  (bind _returnvalue (`|SpawnActorFromClass` "/Game/MapComponents/Spawn/SpawnCamera.SpawnCamera_C" (`KismetMathLibrary.MakeTransform` _returnvalue_location _returnvalue_rotation) "Undefined" "OverrideRootScale"))
  (`CameraComponent.SetFieldOfView` (`/Game/MapComponents/Spawn/SpawnCamera.Camera` _returnvalue) (`self.CameraFOV`))
  (`self.Possess` _returnvalue)
  (`self.FadeCam` 1.0 0.0))

(event `self.ReceiveEndPlay`
  (params (EndPlayReason :type "EEndPlayReason Enum" :default "Destroyed"))
  (`/Engine/EditorBlueprintResources/ActorMacros.Switch Has Authority`
    (:`Remote`
      (`DestroySessionCallbackProxy.DestroySession` self))))

(event `self.ReceiveBeginPlay`
  (`/Game/Blueprints/BP/Library/Object_Macro_Library.IsLocalController`
    (:`true`
      (`self.EnableInput` self))))

(event `InterpFOV`
  (params (FOV :type "Float (double-precision)"))
  (bind _returnvalue (`GameplayStatics.GetWorldDeltaSeconds`))
  ;[1 1 1] Интерполяция FOV
  (`/Game/Blueprints/BP/Library/Actor_Macro_Library.DoWithDelay` _returnvalue :!label _label
    (:`then`
      (set `self.CameraFOV` (`KismetMathLibrary.FInterpTo` (`self.CameraFOV`) FOV _returnvalue 15.0))
      (`self.ChangeFOV`)
      (if (`KismetMathLibrary.NearlyEqual_FloatFloat` FOV (`self.CameraFOV`) 0.0001)
        (goto _label :!via `Break`)))
    (:`OnBreak`
      (set `self.CameraFOV` FOV)
      (`self.ChangeFOV`))))

(fn `ChangeFOV`
  (bind _returnvalue (`self.K2_GetPawn`))
  (bind _asshooter_character (cast `/Game/Character/ShooterCharacter` _returnvalue)
    (:`then`
      (`CameraComponent.SetFieldOfView` (`/Game/Character/ThirdPersonCharacterAnim.Camera` _asshooter_character) (`self.CameraFOV`)))
    (:`CastFailed`
      (bind _asspawn_camera (cast `/Game/MapComponents/Spawn/SpawnCamera` _returnvalue))
      (`CameraComponent.SetFieldOfView` (`/Game/MapComponents/Spawn/SpawnCamera.Camera` _asspawn_camera) (`self.CameraFOV`)))))

(fn `CreateScoreList`
  (`/Engine/EditorBlueprintResources/StandardMacros.IsValid` (`self.ScoreWB`)
    (:`Is Valid`
      (if (`Widget.IsInViewport` (`self.ScoreWB`))
        (`Widget.SetVisibility` (`self.ScoreWB`) "Visible")
        (else
          (`UserWidget.AddToViewport` (`self.ScoreWB`) 0 :!label _label))))
    (:`Is Not Valid`
      (bind _returnvalue (`|CreateWidget` "/Game/UMG/InGameInterface/ScoreBoard.ScoreBoard_C"))
      (set `self.ScoreWB` _returnvalue)
      (goto _label))))

(fn `GetPlayerSettings`
  (params (SlotName :type String :default "PlayerSettings"))
  (returns (GameSave :type "/Game/Blueprints/Settings/PlayerGameSave Object Reference"))
  (locals (_SlotName :type String) (_GameSave :type "/Game/Blueprints/Settings/PlayerGameSave Object Reference"))
  (bind _output_get (set `local._SlotName` SlotName))
  (bind _returnvalue (`GameplayStatics.DoesSaveGameExist` _output_get)) ; Существует ли сохранение с текущим именем
  (if _returnvalue
    (bind _returnvalue_2 (`GameplayStatics.LoadGameFromSlot` (`local._SlotName`))) ; Загружает сохранение
    (set `local._GameSave` (cast `/Game/Blueprints/Settings/PlayerGameSave` _returnvalue_2 :!pure true))
    (else
      (bind _returnvalue_3 (`GameplayStatics.CreateSaveGameObject` "/Game/Blueprints/Settings/PlayerGameSave.PlayerGameSave_C")) ; Создаёт файл сохранения
      (set `local._GameSave` (cast `/Game/Blueprints/Settings/PlayerGameSave` _returnvalue_3 :!pure true))
      (set `/Game/Blueprints/Settings/PlayerGameSave.Settings` (make `/Game/Blueprints/Settings/PlayerSettings` "/Game/Items/Weapon/Primary/AKM/AKM_BP.AKM_BP_C" "/Game/Items/Weapon/Secondary/M9/M9_BP.M9_BP_C" "/Game/Items/Clotch/Hats/Hair_1/Hat_Hair.Hat_Hair_C" "/Game/Items/Clotch/Glasses/Glasses_Master_BP.Glasses_Master_BP_C" "/Game/Items/Clotch/Tops/ACU_Rolled_Up/Top_ACU_Rolled_Up.Top_ACU_Rolled_Up_C" "/Game/Items/Clotch/Gloves/Gloves_Master_BP.Gloves_Master_BP_C" "/Game/Items/Clotch/Pants/TacticalResponse/Pants_TacticalResponse.Pants_TacticalResponse_C" "/Game/Items/Clotch/Shoes/Canvas/Shoes_Canvas.Shoes_Canvas_C") (`local._GameSave`))
      (`/Game/Blueprints/BP/Library/Object_Macro_Library.SavePlayerSettings` (`local._GameSave`) (`local._SlotName`))))
  (return (`local._GameSave`)))

(fn `OnPlayerSpawn`
  (`/Engine/EditorBlueprintResources/StandardMacros.IsValid` (`self.WB_SpawnMenu`)
    (:`Is Valid`
      (`Widget.RemoveFromParent` (`self.WB_SpawnMenu`)))
    (:`Is Not Valid`
      _))
  (`WidgetBlueprintLibrary.SetInputMode_GameOnly` self)
  (`/Game/Blueprints/BP/Library/BP_Funtion_Library.ShowMouseCursor` false))

(fn `SetGamemode`
  (params (Gamemode :type "/Game/Blueprints/BP/ENUMS/E_Gamemods Enum"))
  (bind _asshooter_gameinstance (cast `/Game/Blueprints/ShooterGameinstance` (`GameplayStatics.GetGameInstance`)))
  (set `/Game/Blueprints/ShooterGameinstance.Gamemode` Gamemode _asshooter_gameinstance))

(fn `ShowAftermathUMG`
  (params (WinnerText :type Text))
  (`WidgetLayoutLibrary.RemoveAllWidgets`)
  (bind _returnvalue (`|CreateWidget` "/Game/UMG/InGameInterface/AftermathInfo.AftermathInfo_C" self WinnerText))
  (`UserWidget.AddToViewport` _returnvalue 0))

(fn `ShowRespawnMenu`
  (`/Engine/EditorBlueprintResources/StandardMacros.IsValid` (`self.WB_SpawnMenu`)
    (:`Is Valid`
      _)
    (:`Is Not Valid`
      (bind _returnvalue (`|CreateWidget` "/Game/UMG/Menu/SpawnMenu.SpawnMenu_C" self))
      (set `self.WB_SpawnMenu` _returnvalue)))
  (`UserWidget.AddToViewport` (`self.WB_SpawnMenu`) 0)
  (set `self.bShowMouseCursor` true))

(fn `UserConstructionScript`
  (bind (_gamesettings_sensetivity _gamesettings_mouse_inverse_y) (break `/Game/Blueprints/Settings/GameSettings` (`/Game/Blueprints/Settings/PlayerGameSave.GameSettings` (`self.GetPlayerSettings` "PlayerSettings"))))
  (set `self.Sensetivity` _gamesettings_sensetivity)
  (set `self.MouseInverse` _gamesettings_mouse_inverse_y)
  (`self.ChangeFOV`))