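; Blueprint function library of shared helpers for the multiplayer shooter.
; Match, map and menu helpers route through ShooterGameinstance or the lobby and shooter player controllers, alongside loading screen, cursor and sound-mix volume utilities.
; Small math helpers return point distance and hit trace endpoints.
; Scoreboard sorting orders player states by kills, then regroups equal-kill players by ascending deaths to break ties.
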(fn `GetDistanceBetweenPoints`
  (params (`End Point` :type "Vector Structure") (`Start Point` :type "Vector Structure"))
  (returns (Distance :type "Float (double-precision)"))
  (bind (_returnvalue_x _returnvalue_y _returnvalue_z) (`KismetMathLibrary.BreakVector` (- `End Point` `Start Point`)))
  (return (`KismetMathLibrary.Sqrt` (+ (`KismetMathLibrary.Square` _returnvalue_x) (`KismetMathLibrary.Square` _returnvalue_y) (`KismetMathLibrary.Square` _returnvalue_z)))))

(fn `GetHitStartAndEnd`
  (params (Hit :type "HitResult Structure"))
  (returns (Start :type "Vector Structure") (End :type "Vector Structure"))
  (bind (_bblockinghit _binitialoverlap _time _location _impactpoint _normal _impactnormal _physmat _hitactor _hitcomponent _hitbonename _hititem _faceindex _tracestart _traceend) (`GameplayStatics.BreakHitResult` Hit))
  (return _tracestart (`KismetMathLibrary.SelectVector` _location _traceend _bblockinghit)))

(fn `GetMapByID`
  (params (ID :type Integer))
  (returns (Map :type "/Game/Maps/Map_Struct Structure"))
  (bind _asshooter_gameinstance (cast `/Game/Blueprints/ShooterGameinstance` (`GameplayStatics.GetGameInstance` null)))
  (return (`KismetArrayLibrary.Array_Get` (`/Game/Blueprints/ShooterGameinstance.MapList` _asshooter_gameinstance) ID)))

(fn `GetPlayerStateKillsAndDeaths`
  (params (States :type "Array of /Game/Blueprints/InGame/ShooterPlayerState Object Reference"))
  (returns (Kills :type "Array of Integer") (Deaths :type "Array of Integer"))
  (locals (_Kills :type "Array of Integer") (_Deaths :type "Array of Integer"))
  (for _array_element States
    (`KismetArrayLibrary.Array_Add` (`local._Kills`) (`/Game/Blueprints/InGame/ShooterPlayerState.Kills` _array_element))
    (`KismetArrayLibrary.Array_Add` (`local._Deaths`) (`/Game/Blueprints/InGame/ShooterPlayerState.Deaths` _array_element)))
  (return (`local._Kills`) (`local._Deaths`)))

(fn `LeaveMatch`
  (params (PlayerController :type "PlayerController Object Reference"))
  (bind _asshooter_gameinstance (cast `/Game/Blueprints/ShooterGameinstance` (`GameplayStatics.GetGameInstance` PlayerController)))
  (`/Game/Blueprints/ShooterGameinstance.LeaveGame` _asshooter_gameinstance PlayerController))

(fn `QuitFromMenues`
  (params (Owner :type "Object Object Reference") (CalledFrom :type "/Game/Blueprints/BP/ENUMS/E_CalledFrom Enum"))
  (locals (_Owner :type "Object Object Reference"))
  (set `local._Owner` Owner)
  (switch `/Game/Blueprints/BP/ENUMS/E_CalledFrom` CalledFrom
    (:`NewEnumerator0`
      (bind _asshooter_gameinstance (cast `/Game/Blueprints/ShooterGameinstance` (`GameplayStatics.GetGameInstance` null)))
      (`/Game/Blueprints/ShooterGameinstance.ShowMainMenu` _asshooter_gameinstance))
    (:`NewEnumerator1`
      (bind _aslobby_player_controller (cast `/Game/Blueprints/Menues/LobbyPlayerController` (`local._Owner`)))
      (`/Game/Blueprints/Menues/LobbyPlayerController.SetupLobbyMenu` _aslobby_player_controller))
    (:`NewEnumerator2`
      (bind _asshooter_pc (cast `/Game/Blueprints/InGame/ShooterPC` (`local._Owner`)))
      (`/Game/Blueprints/InGame/ShooterPC.ShowRespawnMenu` _asshooter_pc))))

(fn `SetVolume`
  (params (InSoundClass :type "SoundClass Object Reference") (Volume :type "Float (double-precision)"))
  (`GameplayStatics.SetSoundMixClassOverride` null "/Game/Sounds/Classes/SoundMixMod.SoundMixMod" InSoundClass Volume 1.0 0.2)
  (`GameplayStatics.PushSoundMixModifier` null "/Game/Sounds/Classes/SoundMixMod.SoundMixMod"))

(fn `ShowLoadingScreen`
  (params (OwningPlayer :type "PlayerController Object Reference") (Image :type "Texture2D Object Reference") (Text :type Text))
  (`WidgetLayoutLibrary.RemoveAllWidgets` OwningPlayer)
  (`self.ShowMouseCursor` false OwningPlayer)
  (bind _returnvalue (`|CreateWidget` "/Game/UMG/LoadingScreen.LoadingScreen_C" OwningPlayer Image Text))
  (`UserWidget.AddToViewport` _returnvalue 0)
  (`WidgetBlueprintLibrary.SetInputMode_UIOnlyEx` OwningPlayer _returnvalue))

(fn `ShowMouseCursor`
  (params (bShow :type Boolean))
  (set `PlayerController.bShowMouseCursor` bShow (`GameplayStatics.GetPlayerController` null)))

(fn `SortPlayerStateArray`
  (params (States :type "Array of /Game/Blueprints/InGame/ShooterPlayerState Object Reference"))
  (returns (SortedArray :type "Array of /Game/Blueprints/InGame/ShooterPlayerState Object Reference"))
  (locals (_SortedByKill :type "Array of /Game/Blueprints/InGame/ShooterPlayerState Object Reference") (_States :type "Array of /Game/Blueprints/InGame/ShooterPlayerState Object Reference") (_SortedByDeath :type "Array of /Game/Blueprints/InGame/ShooterPlayerState Object Reference") (_Kills :type "Array of Integer") (_Value :type Integer) (_Deaths :type "Array of Integer") (_KillsSort :type "Array of Integer") (_DeathArr :type "Array of Integer") (_Sort :type "Array of /Game/Blueprints/InGame/ShooterPlayerState Object Reference"))
  (bind (_kills _deaths) (`self.GetPlayerStateKillsAndDeaths` (`local._SortedByKill`)))
  (bind _output_get (set `local._States` States)) ; Изначальный массив
  (bind (_maxvalues _maxindex) (`/Game/Blueprints/BP/Library/Get_Library.GetSortedIntArray` (`self.GetPlayerStateKillsAndDeaths` _output_get)))
  (for _array_element _maxindex
    (`KismetArrayLibrary.Array_Add` (`local._SortedByKill`) (`KismetArrayLibrary.Array_Get` (`local._States`) _array_element)))
  (bind _output_get_2 (set `local._Kills` _kills))
  (set `local._KillsSort` _output_get_2)
  (set `local._Deaths` _deaths)
  (while (!= (`KismetArrayLibrary.Array_Length` (`local._KillsSort`)) 0)
    (`KismetArrayLibrary.Array_Clear` (`local._Sort`))
    (`KismetArrayLibrary.Array_Clear` (`local._DeathArr`))
    (set `local._Value` (`/Game/Blueprints/BP/Library/Get_Library.GetMaxIntOfArray` (`local._KillsSort`)))
    (`KismetArrayLibrary.Array_RemoveItem` (`local._KillsSort`) (`local._Value`))
    (for _array_element_2 (`/Game/Blueprints/BP/Library/Get_Library.GetAllEqualInOfArray` (`local._Kills`) (`local._Value`))
      (`KismetArrayLibrary.Array_Add` (`local._DeathArr`) (`KismetArrayLibrary.Array_Get` (`local._Deaths`) _array_element_2))
      (`KismetArrayLibrary.Array_Add` (`local._Sort`) (`KismetArrayLibrary.Array_Get` (`local._SortedByKill`) _array_element_2)))
    (bind (_maxvalues_2 _maxindex_2 _minvalues _minindex) (`/Game/Blueprints/BP/Library/Get_Library.GetSortedIntArray` (`local._DeathArr`)))
    (for _array_element_3 _minindex
      (`KismetArrayLibrary.Array_Add` (`local._SortedByDeath`) (`KismetArrayLibrary.Array_Get` (`local._Sort`) _array_element_3))))
  (return (`local._SortedByDeath`)))