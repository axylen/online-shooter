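; Base weapon Blueprint for server-authoritative hitscan shooting, with automatic fire, ammo and magazine dropping.
; Shooting sphere-traces from camera aim, or from the gun when blocked or falling, then applies recoil partly seeded by shot count.
; Damage combines distance falloff, bone multipliers from a data table and the victim's clothing defaults, with hitmarkers for characters.
; Multicasts play muzzle, shell and physical-material impact effects; the server requests bullet-hole or traced blood-splatter decals.
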(event `MC_OnShoted`
  (params (Hit :type "HitResult Structure"))
  (`self.OnShoted` Hit))

(event `DropMagazine`
  (bind _returnvalue (`|SpawnActorFromClass` "/Game/Items/Weapon/Magazine.Magazine_C" (`self.GetTransform`) "Undefined" "OverrideRootScale" null (`StaticMeshComponent.StaticMesh` (`self.Magazine`))))
  (`PrimitiveComponent.SetSimulatePhysics` (`/Game/Items/Weapon/Magazine.StaticMesh` _returnvalue) true))

(event `HideMagazine`
  (params (Hide :type Boolean))
  (`SceneComponent.SetHiddenInGame` (`self.Magazine`) Hide false))

(event `ShootDelay`
  (set `self.bShootDelay` false)
  (`/Game/Character/ShooterCharacter.Server_SetShooting` (`self.Character_Ref`) true)
  (`KismetSystemLibrary.Delay` (`self.fShootDelay`))
  (`/Game/Character/ShooterCharacter.Server_SetShooting` (`self.Character_Ref`) false)
  (set `self.bShootDelay` true)
  (if (`self.bAutomatic`)
    (`self.Shooting`))
  (`KismetSystemLibrary.RetriggerableDelay` 0.4)
  (set `self.ShotsInTheRow` 0))

(event `MC_PlayEffects`
  (bind _returnvalue (`GameplayStatics.GetPlayerCharacter` 0))
  (`GameplayStatics.PlaySoundAtLocation` (`self.ShootSound`) (`self.K2_GetActorLocation`) (struct) (`self.RecoilPower`))
  (`GameplayStatics.SpawnEmitterAttached` "/Game/Particles/P_MuzzleFlash.P_MuzzleFlash" (`self.Gun`) "muzzle")
  (bind _returnvalue_2 (`|SpawnActorFromClass` "/Game/Items/Weapon/Sheeve.Sheeve_C" (`KismetMathLibrary.MakeTransform` (`SceneComponent.K2_GetComponentLocation` (`self.Gun`)) (`KismetMathLibrary.RandomRotator` false)) "AlwaysSpawn" "OverrideRootScale" _returnvalue _returnvalue))
  (`PrimitiveComponent.AddForce` (`/Game/Items/Weapon/Sheeve.Sheeve` _returnvalue_2) (+ (* (`SceneComponent.GetForwardVector` (`self.Gun`)) (`KismetMathLibrary.RandomFloatInRange` -200.0 -120.0)) (`KismetMathLibrary.MakeVector` 0.0 0.0 (`KismetMathLibrary.RandomFloatInRange` 200.0 300.0))) "None" false))

(fn `AddAmmoInStack`
  (params (HowMuch :type Integer))
  (set `self.AmmoInStack` (`KismetMathLibrary.Clamp` (+ (`KismetMathLibrary.SelectInt` (`self.MaxAmmo`) HowMuch (== HowMuch 0)) (`self.AmmoInStack`)) 0 (`self.MaxAmmoInStack`))))

(fn `ChangeAmmo`
  (params (Add :type Boolean))
  (if Add
    (if (>= (`self.AmmoInStack`) (- (`self.MaxAmmo`) (`self.CurrentAmmo`)))
      (set `self.AmmoInStack` (- (`self.AmmoInStack`) (- (`self.MaxAmmo`) (`self.CurrentAmmo`))))
      (set `self.CurrentAmmo` (`self.MaxAmmo`))
      (else
        (set `self.CurrentAmmo` (+ (`self.CurrentAmmo`) (`self.AmmoInStack`)))
        (set `self.AmmoInStack` 0)))
    (else
      (set `self.CurrentAmmo` (- (`self.CurrentAmmo`) 1)))))

(fn `ChechIfCanShoot`
  (returns (Can :type Boolean))
  (if (`self.bWantToShoot`)
    (if (`self.bShootDelay`)
      (if (`/Game/Character/ShooterCharacter.bCanShoot` (`self.Character_Ref`))
        (`self.CheckIfHaveAmmo`
          (:`Have`
            (return true))
          (:`Don't Have`
            (return false)))
        (else
          (return false)))
      (else
        (return false)))
    (else
      (return false))))

(fn `Damage`
  (params (Hit :type "HitResult Structure"))
  (locals (BonesArray :type "Array of Name") (_Damage :type "Float (double-precision)"))
  (bind (_bblockinghit _binitialoverlap _time _location _impactpoint _normal _impactnormal _physmat _hitactor _hitcomponent _hitbonename) (`GameplayStatics.BreakHitResult` Hit))
  (bind (_bblockinghit_2 _binitialoverlap_2 _time_2 _location_2 _impactpoint_2 _normal_2 _impactnormal_2 _physmat_2 _hitactor_2 _hitcomponent_2 _hitbonename_2 _hititem _faceindex _tracestart) (`GameplayStatics.BreakHitResult` Hit))
  (`self.MC_OnShoted` Hit)
  (bind (_clothdamagemultipier _clothdamagedecrease _multiplier) (`self.DamageMultiplier` _hitbonename_2 _hitactor_2))
  (set `local._Damage` (`KismetMathLibrary.Conv_IntToDouble` (`KismetMathLibrary.Round` (`KismetMathLibrary.FClamp` (* _clothdamagemultipier (+ (`KismetMathLibrary.Conv_IntToDouble` (* _clothdamagedecrease -1)) (* _multiplier (- (`self.MaxDamage`) (/ (`/Game/Blueprints/BP/Library/BP_Funtion_Library.GetDistanceBetweenPoints` _impactpoint_2 _tracestart) (`self.ShootDistance`)))))) 0.0 (* (`self.MaxDamage`) 3.5)))))
  (cast `/Game/Character/ShooterCharacter` _hitactor
    (:`then`
      (`self.Hitmarker` _hitbonename))
    (:`CastFailed`
      (set `local._Damage` 1.0)))
  (`GameplayStatics.ApplyPointDamage` _hitactor (`local._Damage`) _location Hit (`Pawn.GetController` (`self.Character_Ref`)) self "/Game/Blueprints/BP/DamageTypes/MyDamageType.MyDamageType_C"))

(fn `DamageMultiplier`
  (params (Bone :type Name) (HitActor :type "Actor Object Reference"))
  (returns (ClothDamageMultipier :type "Float (double-precision)") (ClothDamageDecrease :type Integer) (Multiplier :type "Float (double-precision)"))
  (locals (_HitActor :type "/Game/Character/ShooterCharacter Object Reference"))
  (bind ((`Hat_10_788D174F4CE746498BCC59AC4F2A6B70` _hat) (`Glass_14_7A3EE1604F8826EF2BE2DE8DAAF024B0` _glass) (`Top_17_B92402AC4CE8021398089DB25B50EC8D` _top) (`Gloves_20_E1A519C540FD4475D500D89B21480DC0` _gloves) (`Pants_23_52E1915E4A1A7D0C25B50ABF554D3C2B` _pants) (`Shoes_26_57130A4C4D5DCEFBFA25C0856619EEF3` _shoes)) (break `/Game/Blueprints/Settings/PlayerSettings` (`/Game/Character/ShooterCharacter.PlayerSettings` (`local._HitActor`))))
  (bind _asshooter_character (cast `/Game/Character/ShooterCharacter` HitActor)
    (:`then`
      (set `local._HitActor` _asshooter_character)
      (bind _returnvalue (`|GetDataTableRow` "/Game/DataTables/DamageMPTable.DamageMPTable" Bone)
        (:`then`
          (bind (_multiplier _clothtype) (break `/Game/DataTables/Struct_ClothDamageMP` _returnvalue))
          (bind (_damagedecrease _damagemultipier) (defaults `/Game/Items/Weapon/Weapon_Master_BP` (select `/Game/Items/Clotch/E_Clotch` _clothtype :`NewEnumerator0` _hat :`NewEnumerator1` _top :`NewEnumerator2` _gloves :`NewEnumerator3` _glass :`NewEnumerator4` _pants :`NewEnumerator5` _shoes :`NewEnumerator6` "/Game/Items/Clotch/Cloth_Master_BP.Cloth_Master_BP_C" :!type "/Game/Items/Clotch/Cloth_Master_BP Class Reference")))
          (return _damagemultipier _damagedecrease _multiplier))
        (:`RowNotFound`
          (return 1.0 0 1.0))))
    (:`CastFailed`
      (return 1.0 0 1.0))))

(fn `GetDecalMat`
  (params (PhysMat :type "/Game/Materials/PhysicsMaterials/PhysMatSettings Object Reference"))
  (returns (Item :type "MaterialInstance Object Reference"))
  (return (`/Game/Blueprints/BP/Library/Object_Macro_Library.GetRandomItemOfArray` (`/Game/Materials/PhysicsMaterials/PhysMatSettings.DecalMat` PhysMat))))

(fn `GetShootingVectors`
  (returns (Start :type "Vector Structure") (End :type "Vector Structure"))
  (bind _character_ref (`self.Character_Ref`))
  (bind _gun (`self.Gun`))
  (bind _returnvalue (`SceneComponent.K2_GetComponentLocation` (`/Game/Character/ThirdPersonCharacterAnim.CameraColl` (`self.Character_Ref`))))
  (bind _returnvalue_2 (+ (* (`KismetMathLibrary.GetForwardVector` (`Pawn.GetBaseAimRotation` (`self.Character_Ref`))) (`/Game/Blueprints/BP/Library/BP_Funtion_Library.GetDistanceBetweenPoints` (`SceneComponent.GetSocketLocation` (`self.Gun`) "muzzle") _returnvalue)) _returnvalue))
  (bind _returnvalue_3 (* (+ (/ (`KismetMathLibrary.Conv_IntToDouble` (`self.ShotsInTheRow`)) 10.0) (/ (`KismetMathLibrary.VSize` (`self.GetVelocity` _character_ref)) 430.0)) (`self.Spreading`) (`KismetMathLibrary.SelectFloat` 0.25 1.0 (`/Game/Character/ThirdPersonCharacterAnim.Aiming` _character_ref))))
  (bind _returnvalue_4 (* (+ (/ (`KismetMathLibrary.Conv_IntToDouble` (`self.ShotsInTheRow`)) 10.0) (/ (`KismetMathLibrary.VSize` (`self.GetVelocity` (`self.Character_Ref`))) 0.0)) (`self.Spreading`) 0.0))
  (bind _returnvalue_5 (* _returnvalue_3 -1.0))
  (bind _returnvalue_6 (* _returnvalue_4 -1.0))
  (bind (_blockedf _blocked) (`/Game/Character/ShooterCharacter.HandsIK` (`self.Character_Ref`)))
  (if (or _blocked (`NavMovementComponent.IsFalling` (`Character.CharacterMovement` (`self.Character_Ref`))))
    (return (`SceneComponent.K2_GetComponentLocation` _gun) (`KismetMathLibrary.GreaterGreater_VectorRotator` (* (`SceneComponent.GetRightVector` _gun) 15000) (`KismetMathLibrary.MakeRotator` (`KismetMathLibrary.RandomFloatInRange` _returnvalue_6 _returnvalue_4) 0.0 (`KismetMathLibrary.RandomFloatInRange` _returnvalue_6 _returnvalue_4))))
    (else
      (return _returnvalue_2 (`KismetMathLibrary.GreaterGreater_VectorRotator` (+ _returnvalue_2 (* (`KismetMathLibrary.GetForwardVector` (`Pawn.GetBaseAimRotation` (`self.Character_Ref`))) 15000)) (`KismetMathLibrary.MakeRotator` (`KismetMathLibrary.RandomFloatInRange` _returnvalue_5 _returnvalue_3) 0.0 (`KismetMathLibrary.RandomFloatInRange` _returnvalue_5 _returnvalue_3)))))))

(fn `Hitmarker`
  (params (HitBone :type Name))
  (bind _character_ref (`self.Character_Ref`)
    (:`then`
      (`/Game/Character/ShooterCharacter.Owning_ShotHited` _character_ref (== HitBone "head")))
    (:`else`)))

(fn `MakeShot`
  (params (Start :type "Vector Structure") (End :type "Vector Structure"))
  (bind (_outhit _returnvalue) (`KismetSystemLibrary.SphereTraceSingle` Start End 1.0 "TraceTypeQuery4" true (`|MakeArray` (`self.GetOwner`))))
  (if _returnvalue
    (`self.Damage` _outhit)))

(fn `OnShoted`
  (params (Hit :type "HitResult Structure"))
  (locals (_Hit :type "HitResult Structure") (_PhysMat :type "/Game/Materials/PhysicsMaterials/PhysMatSettings Object Reference"))
  (bind (__hit_bblockinghit __hit_binitialoverlap __hit_time __hit_location __hit_impactpoint __hit_normal __hit_impactnormal __hit_physmat __hit_hitactor __hit_hitcomponent) (`GameplayStatics.BreakHitResult` (`local._Hit`)))
  (bind (_start _end) (`/Game/Blueprints/BP/Library/BP_Funtion_Library.GetHitStartAndEnd` (`local._Hit`)))
  (bind _shotedsound (`/Game/Materials/PhysicsMaterials/PhysMatSettings.ShotedSound` (`local._PhysMat`)))
  (bind _shotedparticle (`/Game/Materials/PhysicsMaterials/PhysMatSettings.ShotedParticle` (`local._PhysMat`)))
  (bind _output_get (set `local._Hit` Hit))
  (bind _asphys_mat_settings (cast `/Game/Materials/PhysicsMaterials/PhysMatSettings` (`.PhysMat` (`GameplayStatics.BreakHitResult` _output_get))))
  (set `local._PhysMat` _asphys_mat_settings)
  (`|ExecutionSequence`
    (:`then_0`
      (`/Engine/EditorBlueprintResources/StandardMacros.IsValid` _shotedsound
        (:`Is Valid`
          (`GameplayStatics.PlaySoundAtLocation` _shotedsound (`.End` (`/Game/Blueprints/BP/Library/BP_Funtion_Library.GetHitStartAndEnd` (`local._Hit`)))) ; Звук попадания
        )))
    (:`then_1`
      (`/Engine/EditorBlueprintResources/StandardMacros.IsValid` _shotedparticle
        (:`Is Valid`
          (`GameplayStatics.SpawnEmitterAtLocation` _shotedparticle (`.End` (`/Game/Blueprints/BP/Library/BP_Funtion_Library.GetHitStartAndEnd` (`local._Hit`)))) ; Частицы в месте попадания патрона
        )))
    (:`then_2`
      (`/Engine/EditorBlueprintResources/ActorMacros.Switch Has Authority`
        (:`Authority`
          (if (> (`KismetArrayLibrary.Array_Length` (`/Game/Materials/PhysicsMaterials/PhysMatSettings.DecalMat` (`local._PhysMat`))) 0)
            (if (`|EnumEquality` (`PhysicalMaterial.SurfaceType` (`local._PhysMat`)) "SurfaceType1")
              (bind (_outhit _returnvalue) (`KismetSystemLibrary.SphereTraceSingle` _end (+ _end (* (`KismetMathLibrary.GetDirectionUnitVector` _start _end) 300.0)) 5.0 "TraceTypeQuery1" true))
              (if _returnvalue
                (bind (_bblockinghit _binitialoverlap _time _location _impactpoint _normal _impactnormal _physmat _hitactor _hitcomponent) (`GameplayStatics.BreakHitResult` _outhit))
                (`/Game/Character/ShooterCharacter.MC_SpawnShotDecal` (`self.Character_Ref`) "/Game/Materials/Decals/Blood/BloodDecal.BloodDecal_C" _impactpoint (`KismetMathLibrary.Conv_VectorToRotator` _normal) (`self.GetDecalMat` (`local._PhysMat`)) _hitcomponent))
              (else
                (`/Game/Character/ShooterCharacter.MC_SpawnShotDecal` (`self.Character_Ref`) "/Game/Materials/Decals/BulletHoles/BulletHoleDecal.BulletHoleDecal_C" __hit_impactpoint (`KismetMathLibrary.Conv_VectorToRotator` __hit_normal) (`self.GetDecalMat` (`local._PhysMat`)) __hit_hitcomponent)))))))))

(fn `Recoil`
  (returns (Yaw :type "Float (double-precision)") (Pitch :type "Float (double-precision)"))
  (locals (_Random :type "Float (double-precision)" :default 0.2))
  (bind __random (`local._Random`))
  (bind _recoilpower (`self.RecoilPower`))
  (bind __random_2 (`local._Random`))
  (return (+ (`KismetMathLibrary.RandomFloatInRange` (* -1.0 __random_2) __random_2) (* (`KismetMathLibrary.RandomFloatInRangeFromStream` -0.3 0.4 (`KismetMathLibrary.MakeRandomStream` (`self.ShotsInTheRow`))) _recoilpower)) (+ (* _recoilpower (`KismetMathLibrary.RandomFloatInRangeFromStream` -0.4 0.25 (`KismetMathLibrary.MakeRandomStream` (- (`self.MaxAmmo`) (`self.ShotsInTheRow`))))) (`KismetMathLibrary.RandomFloatInRange` (* -1.0 __random) __random))))

(fn `Shooting`
  (bind (_yaw _pitch) (`self.Recoil`))
  (`/Engine/EditorBlueprintResources/ActorMacros.Switch Has Authority`
    (:`Authority`
      (if (`self.ChechIfCanShoot`)
        (bind (_start _end) (`self.GetShootingVectors`))
        (`self.MakeShot` _start _end)
        (`/Game/Character/ShooterCharacter.AddRecoil` (`self.Character_Ref`) _yaw _pitch)
        (`/Game/Character/ShooterCharacter.CameraShake` (`self.Character_Ref`) "/Game/Blueprints/BP/Shake/Shake_OnShot.Shake_OnShot_C" (`self.RecoilPower`))
        (`self.ChangeAmmo` false)
        (`/Engine/EditorBlueprintResources/StandardMacros.IncrementInt` (`self.ShotsInTheRow`)
          (:`  `
            (`self.MC_PlayEffects`)
            (`self.ShootDelay`)))
        (else
          (`/Game/Character/ShooterCharacter.Server_SetShooting` (`self.Character_Ref`) false))))))

(fn `UserConstructionScript`)

(fn `WantToShoot`
  (params (bWantToShoot :type Boolean))
  (`/Engine/EditorBlueprintResources/ActorMacros.Switch Has Authority`
    (:`Authority`
      (bind _output_get (set `self.bWantToShoot` bWantToShoot))
      (if _output_get
        (`self.Shooting`)))))